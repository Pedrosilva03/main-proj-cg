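; Photoshoot actor that captures a set number of screenshots of a target Object with bounding-box labels, as an image dataset.
; BeginPlay switches the view to a CineCamera, then repeatedly moves it to a random orbit point facing the Object and fires HighResShot.
; Before each shot, ConfigLabels projects the bounds' eight corners to screen, normalises min/max by a hard-coded resolution, and saves them with ObjectID to a hard-coded local path.
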(event Custom|LoopCapture
  (Transformation|SetWorldLocation (Variables|Default|GetCineCamera) (- (Transformation|GetWorldLocation (Variables|/Script/Engine.Actor|GetRootComponent (Variables|Default|GetObject))) (* (Math|Vector|GetForwardVector (Math|Rotator|MakeRotator 0.0 (Math|Random|RandomFloatinRange -6e+01 -2e+01) (Math|Random|RandomFloatinRange -1.8e+02 1.8e+02))) (Math|Random|RandomFloatinRange 2e+02 3e+02))) false true)
  (Transformation|SetWorldRotation (Variables|Default|GetCineCamera) (Math|Rotator|FindLookatRotation (Transformation|GetWorldLocation (Variables|Default|GetCineCamera)) (Transformation|GetWorldLocation (Variables|/Script/Engine.Actor|GetRootComponent (Variables|Default|GetObject)))) false false)
  (Utilities|FlowControl|Delay 0.2)
  (CallFunction|ConfigLabels)
  (Utilities|FlowControl|Delay 0.2)
  (Development|ExecuteConsoleCommand (Utilities|String|Append "HighResShot 1 filename=img_" (Utilities|String|ToString(Integer) (+ (Variables|Default|GetID) (Variables|Default|GetCounter)))) 0))

(event Custom|SetupSystem
  (Game|Player|SetViewTargetwithBlend (Game|GetPlayerController 0) (Components|GetOwner (Variables|Default|GetCineCamera)) 0.0 "VTBlend_Linear" 0.0 false))

(event Custom|ConfigLabels
  (bind _object (Variables|Default|GetObject))
  (bind (_origin _boxextent) (Collision|GetActorBounds _object false false))
  (bind (_x _y _z) (Math|Vector|BreakVector _boxextent))
  (Variables|Default|Setorigin _origin)
  (bind _output_get (Variables|Default|Setx _x))
  (bind _output_get_2 (Variables|Default|Sety _y))
  (bind _output_get_3 (Variables|Default|Setz _z))
  (Variables|Default|Setx0 (* _output_get -1.0))
  (Variables|Default|Sety0 (* _output_get_2 -1.0))
  (Variables|Default|Setz0 (* _output_get_3 -1.0))
  (Variables|Default|Setxmin 1.0)
  (Variables|Default|Setxmax 0.0)
  (Variables|Default|Setymin 1.0)
  (Variables|Default|Setymax 0.0)
  (Variables|Default|SetBB "")
  (for _array_element (Utilities|Array|MakeArray (+ (Variables|Default|Getorigin) (Math|Vector|MakeVector (Variables|Default|Getx) (Variables|Default|Gety) (Variables|Default|Getz))) (+ (Variables|Default|Getorigin) (Math|Vector|MakeVector (Variables|Default|Getx) (Variables|Default|Gety) (Variables|Default|Getz0))) (+ (Variables|Default|Getorigin) (Math|Vector|MakeVector (Variables|Default|Getx) (Variables|Default|Gety0) (Variables|Default|Getz))) (+ (Variables|Default|Getorigin) (Math|Vector|MakeVector (Variables|Default|Getx) (Variables|Default|Gety0) (Variables|Default|Getz0))) (+ (Variables|Default|Getorigin) (Math|Vector|MakeVector (Variables|Default|Getx0) (Variables|Default|Gety) (Variables|Default|Getz))) (+ (Variables|Default|Getorigin) (Math|Vector|MakeVector (Variables|Default|Getx0) (Variables|Default|Gety) (Variables|Default|Getz0))) (+ (Variables|Default|Getorigin) (Math|Vector|MakeVector (Variables|Default|Getx0) (Variables|Default|Gety0) (Variables|Default|Getz))) (+ (Variables|Default|Getorigin) (Math|Vector|MakeVector (Variables|Default|Getx0) (Variables|Default|Gety0) (Variables|Default|Getz0))))
    (if (.ReturnValue (Class|GameplayStatics|ProjectWorldtoScreen (Game|GetPlayerController 0) _array_element false))
      (Variables|Default|SetBB (Utilities|String|Append (Variables|Default|GetBB) "," (Utilities|String|ToString(Vector2d) (.ScreenPosition (Class|GameplayStatics|ProjectWorldtoScreen (Game|GetPlayerController 0) _array_element false)))))
      (Variables|Default|Setxmin (Math|Float|Min(Float) (Variables|Default|Getxmin) (.X (Math|Vector2D|BreakVector2D (Math|Vector2D|MakeVector2D (/ (.X (Math|Vector2D|BreakVector2D (.ScreenPosition (Class|GameplayStatics|ProjectWorldtoScreen (Game|GetPlayerController 0) _array_element false)))) 1526.0) (/ (.Y (Math|Vector2D|BreakVector2D (.ScreenPosition (Class|GameplayStatics|ProjectWorldtoScreen (Game|GetPlayerController 0) _array_element false)))) 862.0))))))
      (Variables|Default|Setxmax (Math|Float|Max(Float) (Variables|Default|Getxmax) (.X (Math|Vector2D|BreakVector2D (Math|Vector2D|MakeVector2D (/ (.X (Math|Vector2D|BreakVector2D (.ScreenPosition (Class|GameplayStatics|ProjectWorldtoScreen (Game|GetPlayerController 0) _array_element false)))) 1526.0) (/ (.Y (Math|Vector2D|BreakVector2D (.ScreenPosition (Class|GameplayStatics|ProjectWorldtoScreen (Game|GetPlayerController 0) _array_element false)))) 862.0))))))
      (Variables|Default|Setymin (Math|Float|Min(Float) (Variables|Default|Getymin) (.Y (Math|Vector2D|BreakVector2D (Math|Vector2D|MakeVector2D (/ (.X (Math|Vector2D|BreakVector2D (.ScreenPosition (Class|GameplayStatics|ProjectWorldtoScreen (Game|GetPlayerController 0) _array_element false)))) 1526.0) (/ (.Y (Math|Vector2D|BreakVector2D (.ScreenPosition (Class|GameplayStatics|ProjectWorldtoScreen (Game|GetPlayerController 0) _array_element false)))) 862.0))))))
      (Variables|Default|Setymax (Math|Float|Max(Float) (Variables|Default|Getymax) (.Y (Math|Vector2D|BreakVector2D (Math|Vector2D|MakeVector2D (/ (.X (Math|Vector2D|BreakVector2D (.ScreenPosition (Class|GameplayStatics|ProjectWorldtoScreen (Game|GetPlayerController 0) _array_element false)))) 1526.0) (/ (.Y (Math|Vector2D|BreakVector2D (.ScreenPosition (Class|GameplayStatics|ProjectWorldtoScreen (Game|GetPlayerController 0) _array_element false)))) 862.0))))))))
  (Development|PrintString (Utilities|String|JoinStringArray (Utilities|Array|MakeArray (Utilities|String|ToString(Float) (Variables|Default|Getxmin)) (Utilities|String|ToString(Float) (Variables|Default|Getxmax)) (Utilities|String|ToString(Float) (Variables|Default|Getymin)) (Utilities|String|ToString(Float) (Variables|Default|Getymax))) " "))
  (Class|FileWriter|SaveStringtoFile (Utilities|String|Append "C:\\Users\\Pedro\\Desktop\\PEDRO\\escuela\\4 ano\\pcg\\main-proj-cg\\ScenesCPP\\Saved\\Screenshots\\WindowsEditor\\img_" (Utilities|String|ToString(Integer) (+ (Variables|Default|GetCounter) (Variables|Default|GetID))) ".txt") (Utilities|String|Append (Utilities|String|ToString(Integer) (Variables|Default|GetObjectID)) " " (Utilities|String|JoinStringArray (Utilities|Array|MakeArray (Utilities|String|ToString(Float) (Variables|Default|Getxmin)) (Utilities|String|ToString(Float) (Variables|Default|Getxmax)) (Utilities|String|ToString(Float) (Variables|Default|Getymin)) (Utilities|String|ToString(Float) (Variables|Default|Getymax))) " ") "zzz" (Variables|Default|GetBB))))

(event EventTick
  (params (DeltaSeconds :type Float%20%28single-precision%29)))

(event EventBeginPlay
  (CallFunction|SetupSystem)
  (Variables|Default|SetCounter 0)
  (CallFunction|LoopCapture :!label _label)
  (Math|Integer|IncrementInt (Variables|Default|GetCounter)
    (:%20%20
      (if (< (Variables|Default|GetCounter) (Variables|Default|GetPhotoCount))
        (Utilities|FlowControl|Delay 2.0)
        (goto _label)))))

(fn ConstructionScript)