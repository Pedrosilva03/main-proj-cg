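; BP_Pics is an automated photoshoot Blueprint that captures a short burst of screenshots from a cine camera when play begins.
; On BeginPlay it sets the player's view to the camera's owner, then runs a counter-driven Delay loop for a fixed number of shots.
; Each pass nudges the camera by a random, cumulative local X/Y offset and fires the Shot console command.
; Look-at rotation nodes are present but unused.
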(event Custom|LoopCapture
  (Transformation|AddLocalOffset (Variables|Default|GetCineCamera) (Math|Vector|MakeVector (Math|Random|RandomFloatinRange -5e+01 5e+01) (Math|Random|RandomFloatinRange -5e+01 5e+01) 0.0) false true)
  (Development|ExecuteConsoleCommand "Shot" 0))

(event Custom|SetupSystem
  (Game|Player|SetViewTargetwithBlend (Game|GetPlayerController 0) (Components|GetOwner (Variables|Default|GetCineCamera)) 0.0 "VTBlend_Linear" 0.0 false))

(event EventBeginPlay
  (CallFunction|SetupSystem)
  (Variables|Default|SetCounter 0)
  (CallFunction|LoopCapture :!label _label)
  (Math|Integer|IncrementInt (Variables|Default|GetCounter)
    (:%20%20
      (if (< (Variables|Default|GetCounter) 10)
        (Utilities|FlowControl|Delay 0.05)
        (goto _label)))))

(fn ConstructionScript)